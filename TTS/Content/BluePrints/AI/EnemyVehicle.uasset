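; EnemyVehicle is an AI enemy vehicle that patrols between two waypoints and explodes when hit by a projectile.
; From BeginPlay it chains AI MoveTo calls to Waypoint01 and Waypoint02, rotating 180 degrees on each arrival and looping back on success.
; Failed moves have no handler.
; A Box overlap with a Projectile spawns an explosion emitter at the Body's location and scale, then destroys the actor.
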(event OnComponentBeginOverlap(Box)
  (params (OverlappedComponent :type Primitive%20Component%20Object%20Reference) (OtherActor :type Actor%20Object%20Reference) (OtherComp :type Primitive%20Component%20Object%20Reference) (OtherBodyIndex :type Integer) (bFromSweep :type Boolean) (SweepResult :type Hit%20Result%20Structure%20%28by%20ref%29))
  (Utilities|Casting|CastToProjectile OtherActor)
  (Effects|SpawnEmitteratLocation "/Game/tts/StarterContent/Particles/P_Explosion.P_Explosion" (Transformation|GetWorldLocation (Variables|Default|GetBody)) "0, 0, 0" (Transformation|GetWorldScale (Variables|Default|GetBody)))
  (Actor|DestroyActor))

(event EventBeginPlay
  (AI|AIMoveTo self "0, 0, 0" (Variables|Default|GetWaypoint01) 5e+02 false :!label _label
    (:OnSuccess
      (Transformation|AddActorLocalRotation "0.000000,180.000000, 0" false false)
      (AI|AIMoveTo self "0, 0, 0" (Variables|Default|GetWaypoint02) 5.0 false
        (:OnSuccess
          (Transformation|AddActorLocalRotation "0.000000,180.000000, 0" false false)
          (goto _label))))))

(fn ConstructionScript)