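; LevelMarker is an actor Blueprint that runs the match countdown and ends the game.
; Tick uses Delay nodes as throttles, decrementing the Minute and Second variables about once per second.
; When the timer runs out, or shortly after Score equals ten, it adds the GameOver widget, shows the mouse cursor and pauses the game.
; Score is only read here.
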(event EventBeginPlay)

(event Collision|EventActorBeginOverlap
  (params (OtherActor :type Actor%20Object%20Reference)))

(event EventTick
  (params (DeltaSeconds :type Float%20%28single-precision%29))
  (if (== (Variables|Default|GetScore) 10)
    (Utilities|FlowControl|Delay 2.0)
    (bind _returnvalue (UserInterface|CreateWidget "/Game/BluePrints/UMG/GameOver.GameOver_C" :!label _label))
    (UserInterface|Viewport|AddtoViewport _returnvalue 0)
    (Variables|/Script/Engine.PlayerController|SetbShowMouseCursor (Game|GetPlayerController 0) true)
    (Game|SetGamePaused true)
    (else
      (Utilities|FlowControl|Delay 1.0)
      (if (== (Variables|Default|GetSecond) 0)
        (if (== (Variables|Default|GetMinute) 0)
          (goto _label)
          (else
            (Variables|Default|SetMinute (- (Variables|Default|GetMinute) 1))
            (Variables|Default|SetSecond 59)))
        (else
          (Variables|Default|SetSecond (- (Variables|Default|GetSecond) 1)))))))

(fn ConstructionScript)