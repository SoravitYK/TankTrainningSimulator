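; Projectile actor that explodes shortly after its movement stops, pushing nearby objects away.
; On projectile stop it enables physics on its Colli component, waits briefly, then spawns a scaled-up explosion emitter at the Sphere's location.
; It then gathers WorldStatic and Pawn components with a capsule overlap, applies a linear-falloff radial impulse to them, and destroys itself.
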(event OnProjectileStop(ProjectileMovement)
  (params (ImpactResult :type Hit%20Result%20Structure%20%28by%20ref%29))
  (bind _returnvalue (Transformation|GetActorLocation))
  (Physics|SetSimulatePhysics (Variables|Default|GetColli) true)
  (Utilities|FlowControl|Delay 0.2)
  (Effects|SpawnEmitteratLocation "/Game/Particles/P_Explosion.P_Explosion" (Transformation|GetWorldLocation (Variables|Default|GetSphere)) "0, 0, 0" "5.000000,5.000000,5.000000")
  (bind _outcomponents (Class|KismetSystemLibrary|CapsuleOverlapComponents _returnvalue 5e+02 0.0 (Utilities|Array|MakeArray "ObjectTypeQuery1" "ObjectTypeQuery3")))
  (Physics|AddRadialImpulse _outcomponents _returnvalue 5e+02 1e+07 "RIF_Linear" false)
  (Actor|DestroyActor))

(event EventBeginPlay)

(event EventTick
  (params (DeltaSeconds :type Float%20%28single-precision%29)))

(fn ConstructionScript)