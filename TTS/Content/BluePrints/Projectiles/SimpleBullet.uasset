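; SimpleBullet is a physics-driven projectile Blueprint that explodes on hit.
; Each tick it rotates to face the velocity of its CollisionSphere.
; On hit it spawns a scaled-up explosion emitter, applies a radial impulse with linear falloff to components found by a capsule overlap, then destroys itself.
; The overlap handler only checks against instigator and self without acting, and a debug-text branch is unwired.
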(event EventBeginPlay)

(event Collision|EventActorBeginOverlap
  (params (OtherActor :type Actor%20Object%20Reference))
  (if (and (!= OtherActor (Variables|Default|GetInstigator)) (!= OtherActor self))
    _))

(event EventTick
  (params (DeltaSeconds :type Float%20%28single-precision%29))
  (bind _returnvalue (Physics|GetPhysicsLinearVelocity (Variables|Default|GetCollisionSphere) "None"))
  (Transformation|SetActorRotation (Math|Rotator|MakeRotfromX _returnvalue)))

(event Collision|EventHit
  (params (MyComp :type Primitive%20Component%20Object%20Reference) (Other :type Actor%20Object%20Reference) (OtherComp :type Primitive%20Component%20Object%20Reference) (bSelfMoved :type Boolean) (HitLocation :type Vector :default "0, 0, 0") (HitNormal :type Vector :default "0, 0, 0") (NormalImpulse :type Vector :default "0, 0, 0") (Hit :type Hit%20Result%20Structure%20%28by%20ref%29))
  (bind _returnvalue (Transformation|GetActorLocation))
  (Effects|SpawnEmitteratLocation "/Game/Particles/P_Explosion.P_Explosion" (Transformation|GetActorLocation) (Transformation|GetActorRotation) "5.000000,5.000000,5.000000")
  (bind _outcomponents (Class|KismetSystemLibrary|CapsuleOverlapComponents _returnvalue 5e+02 0.0 (Utilities|Array|MakeArray "ObjectTypeQuery8" "ObjectTypeQuery7")))
  (Physics|AddRadialImpulse _outcomponents _returnvalue 5e+02 1e+07 "RIF_Linear" false)
  (Actor|DestroyActor))

(fn ConstructionScript
  (|CallParentFunction))